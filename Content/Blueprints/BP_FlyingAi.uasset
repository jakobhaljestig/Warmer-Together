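; Flying AI pawn that can roam around its spawn point and chase the player, steered by direct movement input.
; On BeginPlay it starts BB_FlyingAI through BP_FlyingAiController and records its start location, then mirrors AiState to the blackboard every tick.
; ChasePlayer closes in, backs off or strafes by distance.
; FindRandomLocation retries for points within the roam radius, and MoveAiToLocation flies horizontally toward a target, reporting arrival.
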(event EventBeginPlay
  (Utilities|FlowControl|Sequence
    (:then_0
      (bind _asbp_flying_ai_controller (Utilities|Casting|CastToBP_FlyingAiController (Pawn|GetController)))
      (bind _output_get (Variables|Default|SetFlying%20Ai%20Ref _asbp_flying_ai_controller))
      (bind _blackboardcomponent (Class|AIController|UseBlackboard _output_get "/Game/AI/BB_FlyingAI.BB_FlyingAI"))
      (bind _output_get_2 (Variables|Default|SetBlackboard%20Component%20Ref _blackboardcomponent))
      (AI|Components|Blackboard|SetValueasObject _output_get_2 (Utilities|Name|MakeLiteralName "FlyingActor") self))
    (:then_1
      (Variables|Default|SetStartLocation (Transformation|GetActorLocation)))))

(event EventTick
  (params (DeltaSeconds :type Float%20%28single-precision%29))
  (AI|Components|Blackboard|SetValueasEnum (Variables|Default|GetBlackboard%20Component%20Ref) (Utilities|Name|MakeLiteralName "FlyingState") (Variables|Default|GetAiState)))

(fn ConstructionScript)

(fn ChasePlayer
  (bind _returnvalue (Game|GetPlayerCharacter 0))
  (bind _returnvalue_2 (Transformation|GetActorLocation))
  (bind _returnvalue_3 (Transformation|GetActorLocation))
  (bind _returnvalue_4 (Transformation|GetActorLocation _returnvalue))
  (bind _returnvalue_5 (Math|Vector|MakeVector (.x _returnvalue_4) (.y _returnvalue_4) (.z _returnvalue_2)))
  (bind _returnvalue_6 (Math|Rotator|FindLookatRotation _returnvalue_3 _returnvalue_5))
  (bind _returnvalue_7 (Math|Rotator|GetRotationXVector (Math|Rotator|MakeRotator 0.0 0.0 (.yaw _returnvalue_6))))
  (switch Utilities|FlowControl|Switch|SwitchonChaseStates (Variables|Default|GetChaseStates)
    (:NewEnumerator0
      (if (> (Transformation|GetDistanceTo (Game|GetPlayerCharacter 0)) (Variables|Default|GetAttackDistance))
        (Pawn|Input|AddMovementInput _returnvalue_7 1.0 false)
        (Transformation|SetActorRotation (Math|Rotator|Lerp(Rotator) (Transformation|GetActorRotation) (Math|Rotator|MakeRotator 0.0 0.0 (.yaw _returnvalue_6)) 0.5))
        (return false)
        (elif (< (Transformation|GetDistanceTo (Game|GetPlayerCharacter 0)) (- (Variables|Default|GetAttackDistance) 5e+02))
          (Pawn|Input|AddMovementInput _returnvalue_7 -1.0 false)
          (else
            (Pawn|Input|AddMovementInput (Math|Vector|GetRightVector (Math|Rotator|FindLookatRotation (Transformation|GetActorLocation) (Transformation|GetActorLocation (Game|GetPlayerCharacter 0)))) 1.0 false)))))))

(fn FindRandomLocation
  (bind _returnvalue (Transformation|GetActorLocation))
  (LocalVariables|SetInt 0)
  (Variables|Default|SetTargetLocation (Math|Vector|MakeVector (+ (.x _returnvalue) (Math|Random|RandomFloatinRange -1e+03 1e+03)) (+ (.y _returnvalue) (Math|Random|RandomFloatinRange -1e+03 1e+03)) (.z _returnvalue)) :!label _label)
  (if (> (Math|Float|Absolute(Float) (Math|Vector|VectorLength (- (Variables|Default|GetStartLocation) (Variables|Default|GetTargetLocation)))) (Variables|Default|GetCanRoamRadius))
    (bind _output_get (LocalVariables|SetInt (+ (LocalVariables|GetInt) 1)))
    (if (< _output_get 10)
      (goto _label)
      (else
        (return (Variables|Default|GetStartLocation))))
    (else
      (return (Variables|Default|GetTargetLocation)))))

(fn MoveAitoLocation
  (params (MoveToLocation :type Vector :default "0, 0, 0") (Threshold :type Float%20%28double-precision%29))
  (bind (_x _y) (Math|Vector|BreakVector MoveToLocation))
  (bind _returnvalue (Transformation|GetActorLocation))
  (bind _returnvalue_2 (Transformation|GetActorLocation))
  (bind _returnvalue_3 (Math|Vector|MakeVector _x _y (.z _returnvalue)))
  (bind _returnvalue_4 (Math|Rotator|FindLookatRotation _returnvalue_2 _returnvalue_3))
  (if (> (Math|Vector|VectorLength (- MoveToLocation (Transformation|GetActorLocation))) Threshold)
    (Pawn|Input|AddMovementInput (Math|Rotator|GetRotationXVector (Math|Rotator|MakeRotator 0.0 0.0 (.yaw _returnvalue_4))) 1.0 true)
    (Transformation|SetActorRotation (Math|Rotator|Lerp(Rotator) (Transformation|GetActorRotation) (Math|Rotator|MakeRotator 0.0 0.0 (.yaw _returnvalue_4)) 0.5 true))
    (return false)
    (else
      (return true))))