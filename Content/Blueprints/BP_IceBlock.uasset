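; BP_IceBlock is an interactable block that the interactor pushes or pulls through BeginPush and EndPush, with a hold-button popup.
; While it moves, Tick box-traces just below its physics constraint and sets IsFalling in PushableProperties when nothing is hit.
; On a hit while falling with upward Z velocity, it plays a thud and clears the flag for the listed surface types, all sharing one sound.
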(event EventBeginPlay)

(event Collision|EventActorBeginOverlap
  (params (OtherActor :type Actor%20Object%20Reference)))

(event EventTick
  (params (DeltaSeconds :type Float%20%28single-precision%29))
  (bind _physicsconstraint (Variables|Default|GetPhysicsConstraint))
  (bind _returnvalue (Transformation|GetWorldLocation _physicsconstraint))
  (if (> (Math|Vector|VectorLength (Transformation|GetVelocity)) 1.0)
    (bind _returnvalue_2 (Class|KismetSystemLibrary|BoxTraceSinglebyProfile _returnvalue (- _returnvalue "0.000000,0.000000,20.000000") "110.000000,110.000000,0.000000" (Transformation|GetActorRotation) "BlockAllDynamic" false 0 "ForOneFrame" true))
    (if (not _returnvalue_2)
      (Variables|/Script/SPM.PushableProperties|SetbIsFalling (Variables|Default|GetPushableProperties) true))))

(event Collision|EventHit
  (params (MyComp :type Primitive%20Component%20Object%20Reference) (Other :type Actor%20Object%20Reference) (OtherComp :type Primitive%20Component%20Object%20Reference) (bSelfMoved :type Boolean) (HitLocation :type Vector :default "0, 0, 0") (HitNormal :type Vector :default "0, 0, 0") (NormalImpulse :type Vector :default "0, 0, 0") (Hit :type Hit%20Result%20Structure%20%28by%20ref%29))
  (if (and (Variables|/Script/SPM.PushableProperties|GetbIsFalling (Variables|Default|GetPushableProperties)) (> (.z (Transformation|GetVelocity)) 1.0))
    (switch Utilities|FlowControl|Switch|SwitchonEPhysicalSurface (Collision|GetSurfaceType Hit)
      (:SurfaceType1
        _)
      (:SurfaceType2
        _)
      (:SurfaceType3
        _)
      (:SurfaceType4
        _)
      (:SurfaceType5
        _))
    (Audio|PlaySoundatLocation "/Game/Audio/SoundWaves/A_thud.A_thud" (Transformation|GetWorldLocation (Variables|Default|GetCube)) "0, 0, 0" 1.0 1.0 0.0 0 0 0 0)
    (Variables|/Script/SPM.PushableProperties|SetbIsFalling (Variables|Default|GetPushableProperties) false)))

(fn ConstructionScript)

(fn EndInteraction
  (params (Interactor :type Character%20Base%20Object%20Reference))
  (Class|CharacterBase|EndPush Interactor)
  (return false))

(fn GetPopupInfo
  (params (Interactor :type Character%20Base%20Object%20Reference))
  (return "Hold To Push/Pull" "/Game/Assets/UI/Buttons/Controller/ButtonX_70x70.ButtonX_70x70"))

(fn Interact
  (params (Interactor :type Character%20Base%20Object%20Reference))
  (Class|CharacterBase|BeginPush Interactor)
  (return false))