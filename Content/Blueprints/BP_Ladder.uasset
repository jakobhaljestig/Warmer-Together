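; BP_Ladder is a procedural ladder whose construction script sizes it from LadderHeight.
; It scales both poles, then loops a helper that adds rotated bar instances to BarsInstance every LadderGap up to the ladder's height.
; Logic for scaling the climbing zone and collider and for placing optional decorative pole-end meshes is present but disconnected.
; Bar transforms are hardcoded to the current meshes.
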(fn ConstructionScript
  (Transformation|SetRelativeScale3D (Variables|Default|GetLeftLadderPole) (Math|Vector|MakeVector 0.1 0.1 (Variables|Default|GetLadder%20Height)))
  (while (< (Variables|Default|GetCompare%20Height) (* (Variables|Default|GetLadder%20Height) 1e+02))
    (Utilities|AddBars&Screws))
  (Utilities|FlowControl|Sequence) ; Till för slutet av stegen
)