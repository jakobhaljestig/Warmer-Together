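; BP_FallingTree12 is an interactable tree that the player pushes by holding a button, shown by a "Hold To Push" popup with an X button icon.
; Interact calls BeginPush on the interactor and EndInteraction calls EndPush, both returning false.
; BeginPlay and the construction script only call their parents, and the file itself holds no falling logic.
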(event EventBeginPlay
  (|CallParentFunction))

(event Collision|EventActorBeginOverlap
  (params (OtherActor :type Actor%20Object%20Reference)))

(fn ConstructionScript
  (|CallParentFunction))

(fn Interact
  (params (Interactor :type Character%20Base%20Object%20Reference))
  (Class|CharacterBase|BeginPush Interactor)
  (return false))

(fn EndInteraction
  (params (Interactor :type Character%20Base%20Object%20Reference))
  (Class|CharacterBase|EndPush Interactor)
  (return false))

(fn GetPopupInfo
  (params (Interactor :type Character%20Base%20Object%20Reference))
  (return "Hold To Push" "/Game/Assets/UI/Buttons/Controller/ButtonX_70x70.ButtonX_70x70"))