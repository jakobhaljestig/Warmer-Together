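; BP_FallingTree is a tree actor whose log topples over after it is hit.
; The Hit event sets a Falling flag, which Tick checks every frame.
; While the flag is set, Tick uses RInterpTo to ease the Log's relative rotation toward a pitch derived from FallingAngle, keeping its current yaw.
; Nothing in the graph clears the flag, so the interpolation keeps running after the fall.
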(event EventBeginPlay)

(event Collision|EventActorBeginOverlap
  (params (OtherActor :type Actor%20Object%20Reference)))

(event EventTick
  (params (DeltaSeconds :type Float%20%28single-precision%29))
  (bind _log (Variables|Default|GetLog))
  (if (Variables|Default|GetFalling)
    (Transformation|SetRelativeRotation (Variables|Default|GetLog) (Math|Interpolation|RInterpTo (Variables|/Script/Engine.SceneComponent|GetRelativeRotation _log) (Math|Rotator|MakeRotator 0.0 (- (Variables|Default|GetFallingAngle) 9e+01) (.yaw (Variables|/Script/Engine.SceneComponent|GetRelativeRotation _log))) DeltaSeconds 5.0) false false)))

(event Collision|EventHit
  (params (MyComp :type Primitive%20Component%20Object%20Reference) (Other :type Actor%20Object%20Reference) (OtherComp :type Primitive%20Component%20Object%20Reference) (bSelfMoved :type Boolean) (HitLocation :type Vector :default "0, 0, 0") (HitNormal :type Vector :default "0, 0, 0") (NormalImpulse :type Vector :default "0, 0, 0") (Hit :type Hit%20Result%20Structure%20%28by%20ref%29))
  (Variables|Default|SetFalling true))

(fn ConstructionScript)