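; BP_MiniGameRadio is an early radio mini-game Blueprint that currently only prints debug output for gamepad face-button input.
; Each of the four face buttons prints its position on press, and Tick prints the MiniGame's RequestedInput every frame.
; The ReadInput calls on MiniGame are left unconnected, so presses are never passed to the mini-game.
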(event EventTick
  (params (DeltaSeconds :type Float%20%28single-precision%29))
  (Development|PrintString (Utilities|String|ToString(Integer) (Variables|/Script/SPM.MiniGame|GetRequestedInput (Variables|Default|GetMiniGame)))))

(event Collision|EventHit
  (params (MyComp :type Primitive%20Component%20Object%20Reference) (Other :type Actor%20Object%20Reference) (OtherComp :type Primitive%20Component%20Object%20Reference) (bSelfMoved :type Boolean) (HitLocation :type Vector :default "0, 0, 0") (HitNormal :type Vector :default "0, 0, 0") (NormalImpulse :type Vector :default "0, 0, 0") (Hit :type Hit%20Result%20Structure%20%28by%20ref%29)))

(event Collision|EventActorBeginOverlap
  (params (OtherActor :type Actor%20Object%20Reference)))

(event Input|GamepadEvents|GamepadFaceButtonTop
  (params (Key :type Key%20Structure :default "None"))
  (:Pressed
    (Development|PrintString "TOP")))

(event Input|GamepadEvents|GamepadFaceButtonLeft
  (params (Key :type Key%20Structure :default "None"))
  (:Pressed
    (Development|PrintString "LEFT")))

(event Input|GamepadEvents|GamepadFaceButtonRight
  (params (Key :type Key%20Structure :default "None"))
  (:Pressed
    (Development|PrintString "RIGHT")))

(event Input|GamepadEvents|GamepadFaceButtonBottom
  (params (Key :type Key%20Structure :default "None"))
  (:Pressed
    (Development|PrintString "BOTTOM")))

(fn ConstructionScript)