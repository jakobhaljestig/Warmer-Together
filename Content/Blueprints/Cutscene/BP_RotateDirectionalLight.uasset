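; Trigger actor that rotates the level's directional light once, for a cutscene sun movement.
; On actor overlap it destroys its trigger so it cannot fire again, then stores the light's current rotation.
; A timeline lerps the light from that stored rotation to the target NewRotation along its curve.
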(event Collision|EventActorBeginOverlap
  (params (OtherActor :type Actor%20Object%20Reference))
  (Components|DestroyComponent (Variables|Default|GetTrigger))
  (Variables|Default|SetOriginalRotation (Transformation|GetActorRotation (Variables|Default|GetDirectionalLight)))
  (bind _newtrack_0 (Timeline|MoveSunTrack Play)
    (:Update
      (Transformation|SetActorRotation (Variables|Default|GetDirectionalLight) (Math|Rotator|Lerp(Rotator) (Variables|Default|GetOriginalRotation) (Variables|Default|GetNewRotation) _newtrack_0)))))

(fn ConstructionScript)