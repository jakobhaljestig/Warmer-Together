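; One-shot trigger box that plays a level sequence cutscene in which both players' characters run along their own splines.
; A timeline, rate-scaled to the sequence's end time less one second, drives each character's position and yaw along its spline.
; Meanwhile it forces single-screen view, disables input, plays run animations and zeroes body-temperature cooldown.
; When the timeline finishes, it restores all of these and turns on InvisibleBlock's query collision.
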(event Collision|EventActorBeginOverlap
  (params (OtherActor :type Actor%20Object%20Reference))
  (bind _returnvalue (Game|GetPlayerCharacter 0))
  (bind _returnvalue_2 (Game|GetPlayerCharacter 1))
  (bind _levelsequenceactor (Variables|Default|GetLevelSequenceActor))
  (bind _sequenceplayer (Variables|/Script/LevelSequence.LevelSequenceActor|GetSequencePlayer _levelsequenceactor))
  (Utilities|Casting|CastToCharacterBase OtherActor)
  (Components|DestroyComponent (Variables|Default|GetTriggerBox))
  (Collision|SetCollisionEnabled (Variables|Default|GetInvisibleBlock) "NoCollision")
  ;[0.15 0.15 0.15 0.5] Change Timeline Length to match Sequencer Duration
  (Components|Timeline|SetPlayRate (Variables|Default|GetFollowSplinesTrack) (/ 1.0 (- (Class|TimeManagementBlueprintLibrary|ToSeconds(QualifiedFrameTime) (Class|MovieSceneSequencePlayer|GetEndTime _sequenceplayer)) 1.0)))
  (Sequencer|Player|Play _sequenceplayer :!class /Script/MovieScene.MovieSceneSequencePlayer)
  (Utilities|FlowControl|Delay 0.5)
  (Class|GameplayStatics|SetForceDisableSplitscreen true)
  ;[0.15 0.15 0.15 0.5] Move Characteres to start of respective Spline and start Run animation
  (CallFunction|MoveCharactertoSpline _returnvalue (Variables|Default|GetSplineBig))
  (CallFunction|MoveCharactertoSpline _returnvalue_2 (Variables|Default|GetSplineSmall))
  (Components|Animation|PlayAnimation (Variables|/Script/Engine.Character|GetMesh _returnvalue) "/Game/Characters/BigCharacter/Animations/AS_BigRunning.AS_BigRunning" true)
  (Components|Animation|PlayAnimation (Variables|/Script/Engine.Character|GetMesh _returnvalue_2) "/Game/Characters/SmallCharacter/Animations/AS_SmallRunning.AS_SmallRunning" true)
  ;[0.15 0.15 0.15 0.5] Zero Cooldown Rate
  (bind _ascharacter_base (Utilities|Casting|CastToCharacterBase _returnvalue))
  (Variables|Default|SetCooldownRateBig (Variables|/Script/SPM.BodyTemperature|GetCoolDownRate (Variables|/Script/SPM.CharacterBase|GetBodyTempComponent _ascharacter_base)))
  (Class|BodyTemperature|SetCoolDownRate (Variables|/Script/SPM.CharacterBase|GetBodyTempComponent _ascharacter_base) 0.0)
  (bind _ascharacter_base_2 (Utilities|Casting|CastToCharacterBase _returnvalue_2))
  (Variables|Default|SetCooldownRateSmall (Variables|/Script/SPM.BodyTemperature|GetCoolDownRate (Variables|/Script/SPM.CharacterBase|GetBodyTempComponent _ascharacter_base_2)))
  (Class|BodyTemperature|SetCoolDownRate (Variables|/Script/SPM.CharacterBase|GetBodyTempComponent _ascharacter_base_2) 0.0)
  (bind (_direction _movetrackbig _movetracksmall) (Timeline|FollowSplinesTrack Play)
    (:Update
      ;[0.15 0.15 0.15 0.5] Characters follow Spline
      (CallFunction|FollowSpline _movetrackbig (Game|GetPlayerCharacter 0) (Variables|Default|GetSplineBig))
      (CallFunction|FollowSpline _movetracksmall (Game|GetPlayerCharacter 1) (Variables|Default|GetSplineSmall)))
    (:Finished
      ;[0.15 0.15 0.15 0.5] Reset Characters after follow Spline
      (Class|GameplayStatics|SetForceDisableSplitscreen false)
      (CallFunction|ResetAfterCutscene (Game|GetPlayerCharacter 0) (Variables|Default|GetCooldownRateBig))
      (CallFunction|ResetAfterCutscene (Game|GetPlayerCharacter 1) (Variables|Default|GetCooldownRateSmall))
      (Collision|SetCollisionEnabled (Variables|Default|GetInvisibleBlock) "QueryOnly"))))

(fn ConstructionScript)

(fn MoveCharactertoSpline
  (params (Character :type Character%20Object%20Reference) (Spline :type Spline%20Component%20Object%20Reference))
  (bind _asbp_character_player_controller (Utilities|Casting|CastToBP_CharacterPlayerController (Pawn|GetController Character)))
  (Input|DisableInput Character _asbp_character_player_controller)
  (Transformation|SetActorLocation Character (Spline|GetLocationatSplinePoint Spline 0 "World") false true))

(fn ResetAfterCutscene
  (params (Character :type Character%20Object%20Reference) (CooldownRate :type Float%20%28double-precision%29))
  (bind _returnvalue (Pawn|GetController Character))
  (Components|Animation|SetAnimationMode (Variables|/Script/Engine.Character|GetMesh Character) "AnimationBlueprint" true)
  (bind _asbp_character_player_controller (Utilities|Casting|CastToBP_CharacterPlayerController _returnvalue))
  (Input|EnableInput Character _asbp_character_player_controller)
  (Pawn|SetControlRotation _returnvalue (Transformation|GetActorRotation Character))
  (bind _ascharacter_base (Utilities|Casting|CastToCharacterBase Character))
  (Class|BodyTemperature|SetCoolDownRate (Variables|/Script/SPM.CharacterBase|GetBodyTempComponent _ascharacter_base) CooldownRate))

(fn FollowSpline
  (params (Alpha :type Float%20%28double-precision%29) (Character :type Character%20Object%20Reference) (Spline :type Spline%20Component%20Object%20Reference))
  (bind _returnvalue (Spline|GetSplineLength Spline))
  (bind _returnvalue_2 (Math|Float|Lerp 0.0 _returnvalue Alpha))
  (Transformation|SetActorLocationAndRotation Character (Spline|GetLocationatDistanceAlongSpline Spline _returnvalue_2 "World") (Math|Rotator|MakeRotator 0.0 0.0 (.yaw (Spline|GetRotationatDistanceAlongSpline Spline _returnvalue_2 "World"))) true))