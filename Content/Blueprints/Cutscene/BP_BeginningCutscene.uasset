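; Actor that runs the opening cutscene for a two-player splitscreen game, then destroys itself.
; TriggerCutscene flags InCutscene on the game instance, starts and immediately pauses the CutsceneBeginning sequence, and force-disables splitscreen.
; ContinueCutscene disables both players' input, hides their HUDs, resets their states and resumes playback.
; Half a second before the sequence's end time, it restores splitscreen, possession, input and HUDs, and clears the flag.
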(event Custom|TriggerCutscene
  (bind _cutscenebeginning (Variables|Default|GetCutsceneBeginning))
  (bind _sequenceplayer (Variables|/Script/LevelSequence.LevelSequenceActor|GetSequencePlayer _cutscenebeginning))
  (bind _asbp_warmer_together_game_instance (Utilities|Casting|CastToBP_WarmerTogetherGameInstance (Game|GetGameInstance)))
  (bind _output_get (Variables|Default|SetAs%20BP%20Warmer%20Together%20Game%20Instance _asbp_warmer_together_game_instance))
  (Variables|/Game/Blueprints/SaveGame/BP_WarmerTogetherGameInstance.BP_WarmerTogetherGameInstance_C|SetInCutscene _output_get true)
  (Sequencer|Player|Play _sequenceplayer :!class /Script/MovieScene.MovieSceneSequencePlayer)
  (Sequencer|Player|Pause _sequenceplayer)
  (Class|GameplayStatics|SetForceDisableSplitscreen true))

(event Custom|ContinueCutscene
  (bind _returnvalue (Game|GetPlayerCharacter 0))
  (bind _returnvalue_2 (Game|GetPlayerCharacter 1))
  (bind _cutscenebeginning (Variables|Default|GetCutsceneBeginning))
  (bind _sequenceplayer (Variables|/Script/LevelSequence.LevelSequenceActor|GetSequencePlayer _cutscenebeginning))
  (CallFunction|DisablePlayerInput _returnvalue)
  (bind _ascharacter_base (Utilities|Casting|CastToCharacterBase _returnvalue))
  (Class|CharacterBase|ResetPlayerState _ascharacter_base)
  (CallFunction|DisablePlayerInput _returnvalue_2)
  (bind _ascharacter_base_2 (Utilities|Casting|CastToCharacterBase _returnvalue_2))
  (Class|CharacterBase|ResetPlayerState _ascharacter_base_2)
  (Sequencer|Player|Play _sequenceplayer :!class /Script/MovieScene.MovieSceneSequencePlayer)
  (Utilities|FlowControl|Delay (- (Class|TimeManagementBlueprintLibrary|ToSeconds(QualifiedFrameTime) (Class|MovieSceneSequencePlayer|GetEndTime _sequenceplayer)) 0.5))
  (Class|GameplayStatics|SetForceDisableSplitscreen false)
  (CallFunction|EnablePlayerInput (Game|GetPlayerCharacter 0))
  (CallFunction|EnablePlayerInput (Game|GetPlayerCharacter 1))
  (Variables|/Game/Blueprints/SaveGame/BP_WarmerTogetherGameInstance.BP_WarmerTogetherGameInstance_C|SetInCutscene (Variables|Default|GetAs%20BP%20Warmer%20Together%20Game%20Instance) false)
  (Actor|DestroyActor))

(fn ConstructionScript)

(fn DisablePlayerInput
  (params (Character :type Character%20Object%20Reference))
  (bind _asbp_character_player_controller (Utilities|Casting|CastToBP_CharacterPlayerController (Pawn|GetController Character)))
  (Input|DisableInput Character _asbp_character_player_controller)
  (Class|CharacterPlayerController|HideHUD _asbp_character_player_controller true))

(fn EnablePlayerInput
  (params (Character :type Character%20Object%20Reference))
  (bind _asbp_character_player_controller (Utilities|Casting|CastToBP_CharacterPlayerController (Pawn|GetController Character)))
  (Input|EnableInput Character _asbp_character_player_controller)
  (Pawn|Possess _asbp_character_player_controller Character)
  (Class|CharacterPlayerController|HideHUD _asbp_character_player_controller false))