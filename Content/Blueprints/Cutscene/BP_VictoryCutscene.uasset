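; BP_VictoryCutscene runs the two-player victory cutscene when TriggerVictory fires, playing a level sequence with helicopter or UFO audio and forcing splitscreen off.
; MovePlayers snaps both players onto victory stand-ins, disables input, hides HUDs and zeroes body-temperature cooldown before wave animations and a music change.
; A timeline keeps players facing the active sequence camera, then pauses the sequence.
; The Alien flag swaps audio, skips rumble and spawns an alien ship above player two.
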(event Custom|TriggerVictory
  (bind _returnvalue (Game|GetPlayerCharacter 1))
  (bind _returnvalue_2 (Game|GetPlayerCharacter 0))
  (bind _returnvalue_3 (Game|GetPlayerCharacter 1))
  (bind _returnvalue_4 (Transformation|GetActorLocation _returnvalue_3))
  (Sequencer|Player|Play (Variables|/Script/LevelSequence.LevelSequenceActor|GetSequencePlayer (Variables|Default|GetLevelSequenceActor)) :!class /Script/MovieScene.MovieSceneSequencePlayer)
  (if (Variables|Default|GetAlien)
    (Audio|Components|Audio|SetSound (Variables|Default|GetHelicopterAudio) "/Game/Audio/SoundWaves/A_ufo-landing.A_ufo-landing"))
  (Audio|Components|Audio|Play (Variables|Default|GetHelicopterAudio) 0.0)
  (Utilities|FlowControl|Delay 0.6)
  (Class|GameplayStatics|SetForceDisableSplitscreen true)
  ;[0.15 0.15 0.15 0.5] Move Players and Start Victory Animation
  (CallFunction|MovePlayers _returnvalue_2 (Variables|Default|GetCharacterBig_Victory))
  (CallFunction|MovePlayers _returnvalue (Variables|Default|GetCharacterSmall_Victory))
  (Components|Animation|PlayAnimation (Variables|/Script/Engine.Character|GetMesh _returnvalue_2) "/Game/Characters/BigCharacter/Animations/AC_BigWaveHelp.AC_BigWaveHelp" true)
  (Components|Animation|PlayAnimation (Variables|/Script/Engine.Character|GetMesh _returnvalue) "/Game/Characters/SmallCharacter/Animations/AC_SmallWaveHelp.AC_SmallWaveHelp" true)
  (bind _asbp_music_manager (Utilities|Casting|CastToBP_MusicManager (Variables|Default|GetMusicManager)))
  (Default|ChangeTrack _asbp_music_manager (Variables|Default|GetTrack))
  (Timeline|LookAtCameraTrack Play
    (:Update
      (CallFunction|LookatCamera (Game|GetPlayerCharacter 0))
      (CallFunction|LookatCamera _returnvalue_3)
      (if (Variables|Default|GetAlien)
        (Game|SpawnActorfromClass "/Game/Blueprints/BP_AlienShip.BP_AlienShip_C" (Math|Transform|MakeTransform (Math|Vector|MakeVector (.x _returnvalue_4) (.y _returnvalue_4) (+ (.z _returnvalue_4) 1e+03)) "0, 0, 0" "1.000000,1.000000,1.000000") "Undefined" "MultiplyWithRoot" 0 0)
        (Variables|Default|SetAlien false)))
    (:Finished
      (Sequencer|Player|Pause (Variables|/Script/LevelSequence.LevelSequenceActor|GetSequencePlayer (Variables|Default|GetLevelSequenceActor))))))

(fn ConstructionScript)

(fn MovePlayers
  (params (PlayerCharacter :type Character%20Object%20Reference) (VictoryCharacter :type Actor%20Object%20Reference))
  (Transformation|SetActorLocationAndRotation PlayerCharacter (Transformation|GetActorLocation VictoryCharacter) (Transformation|GetActorRotation VictoryCharacter))
  (bind _asbp_character_player_controller (Utilities|Casting|CastToBP_CharacterPlayerController (Pawn|GetController PlayerCharacter)))
  (Input|DisableInput PlayerCharacter _asbp_character_player_controller)
  (Class|CharacterPlayerController|HideHUD _asbp_character_player_controller true)
  (if (Variables|Default|GetAlien)
    _
    (else
      (Game|Feedback|ClientPlayForceFeedback _asbp_character_player_controller "/Game/Blueprints/ForceFeedback/FFE_VictoryCutscene.FFE_VictoryCutscene" "None" false false false)))
  (bind _ascharacter_base (Utilities|Casting|CastToCharacterBase PlayerCharacter))
  (Class|BodyTemperature|SetCoolDownRate (Variables|/Script/SPM.CharacterBase|GetBodyTempComponent _ascharacter_base) 0.0))

(fn LookatCamera
  (params (Character :type Character%20Object%20Reference))
  (Transformation|SetActorRotation Character (Math|Rotator|MakeRotator 0.0 0.0 (.yaw (Math|Rotator|FindLookatRotation (Transformation|GetActorLocation Character) (Transformation|GetWorldLocation (Class|LevelSequencePlayer|GetActiveCameraComponent (Variables|/Script/LevelSequence.LevelSequenceActor|GetSequencePlayer (Variables|Default|GetLevelSequenceActor)))))))))