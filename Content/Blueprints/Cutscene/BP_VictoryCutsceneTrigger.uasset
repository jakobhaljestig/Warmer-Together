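; Cutscene trigger Blueprint that stages the two-player victory celebration.
; Victory plays a level sequence, force-disables splitscreen, then calls MovePlayers for player characters 0 and 1.
; MovePlayers snaps each character to its big or small victory stand-in's transform and disables input through BP_CharacterPlayerController.
; Each player's mesh then loops its own chicken dance animation.
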(fn ConstructionScript)

(fn MovePlayers
  (params (PlayerCharacter :type Character%20Object%20Reference) (VictoryCharacter :type Actor%20Object%20Reference))
  (Transformation|SetActorLocationAndRotation PlayerCharacter (Transformation|GetActorLocation VictoryCharacter) (Transformation|GetActorRotation VictoryCharacter))
  (bind _asbp_character_player_controller (Utilities|Casting|CastToBP_CharacterPlayerController (Pawn|GetController PlayerCharacter)))
  (Input|DisableInput PlayerCharacter _asbp_character_player_controller))

(fn Victory
  (bind _returnvalue (Game|GetPlayerCharacter 1))
  (bind _returnvalue_2 (Game|GetPlayerCharacter 0))
  (Sequencer|Player|Play (Variables|/Script/LevelSequence.LevelSequenceActor|GetSequencePlayer (Variables|Default|GetLevelSequenceActor)) :!class /Script/MovieScene.MovieSceneSequencePlayer)
  (Class|GameplayStatics|SetForceDisableSplitscreen true)
  ;[0.15 0.15 0.15 0.5] Move Players and Start Victory Animation
  (CallFunction|MovePlayers _returnvalue_2 (Variables|Default|GetCharacterBig_Victory))
  (Components|Animation|PlayAnimation (Variables|/Script/Engine.Character|GetMesh _returnvalue_2) "/Game/Characters/BigCharacter/Animations/Anim_BigChicken_Dance.Anim_BigChicken_Dance" true)
  (CallFunction|MovePlayers _returnvalue (Variables|Default|GetCharacterSmall_Victory))
  (Components|Animation|PlayAnimation (Variables|/Script/Engine.Character|GetMesh _returnvalue) "/Game/Characters/SmallCharacter/Animations/AS_SmallChickenDance.AS_SmallChickenDance" true))