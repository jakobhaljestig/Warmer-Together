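; BP_Swing is a swing that pitches its Anchor back and forth between positive and negative MaxAngle.
; Each Tick accelerates it up to a maximum until it passes DeaccelerationAngle on the starting side, then slows it, and applies the speed as local rotation.
; Deceleration snaps to MinimumRotationSpeed at a hard-coded threshold, not at that variable's value.
; At each limit, MoveForward flips and speed resets to zero.
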(event EventTick
  (params (DeltaSeconds :type Float%20%28single-precision%29))
  (bind _returnvalue (CallFunction|ShouldAccelerate?))
  (if _returnvalue
    (CallFunction|Accelerate DeltaSeconds)
    (else
      (CallFunction|Deaccelerate DeltaSeconds)))
  (CallFunction|Rotate DeltaSeconds))

(fn ConstructionScript)

(fn Deaccelerate
  (params (DeltaTime :type Float%20%28double-precision%29))
  (if (> (Variables|Default|GetCurrentRotationSpeed) 3e+01)
    (Variables|Default|SetCurrentRotationSpeed (- (Variables|Default|GetCurrentRotationSpeed) (* (Variables|Default|GetRotationDeacceleration) DeltaTime)))
    (else
      (Variables|Default|SetCurrentRotationSpeed (Variables|Default|GetMinimumRotationSpeed)))))

(fn Accelerate
  (params (DeltaTime :type Float%20%28double-precision%29))
  (if (< (Variables|Default|GetCurrentRotationSpeed) (Variables|Default|GetMaxRotationSpeed))
    (Variables|Default|SetCurrentRotationSpeed (+ (Variables|Default|GetCurrentRotationSpeed) (* (Variables|Default|GetRotationAcceleration) DeltaTime)))
    (else
      (Variables|Default|SetCurrentRotationSpeed (Variables|Default|GetMaxRotationSpeed)))))

(fn ShouldAccelerate?
  (return (or (and (>= (.pitch (Transformation|GetWorldRotation (Variables|Default|GetAnchor))) (Variables|Default|GetDeaccelerationAngle)) (not (Variables|Default|GetMoveForward?))) (and (<= (.pitch (Transformation|GetWorldRotation (Variables|Default|GetAnchor))) (* (Variables|Default|GetDeaccelerationAngle) -1.0)) (Variables|Default|GetMoveForward?)))))

(fn Rotate
  (params (DeltaTime :type Float%20%28double-precision%29))
  (bind _anchor (Variables|Default|GetAnchor))
  (if (Variables|Default|GetMoveForward?)
    (Transformation|AddLocalRotation _anchor (Math|Rotator|MakeRotator 0.0 (* DeltaTime (Variables|Default|GetCurrentRotationSpeed)) 0.0) false false)
    (if (>= (.pitch (Transformation|GetWorldRotation (Variables|Default|GetAnchor))) (Variables|Default|GetMaxAngle))
      (Variables|Default|SetMoveForward? false)
      (Variables|Default|SetCurrentRotationSpeed 0.0 :!label _label))
    (else
      (Transformation|AddLocalRotation _anchor (Math|Rotator|MakeRotator 0.0 (* (* (Variables|Default|GetCurrentRotationSpeed) -1.0) DeltaTime) 0.0) false false)
      (if (<= (.pitch (Transformation|GetWorldRotation (Variables|Default|GetAnchor))) (* (Variables|Default|GetMaxAngle) -1.0))
        (Variables|Default|SetMoveForward? true)
        (goto _label)))))