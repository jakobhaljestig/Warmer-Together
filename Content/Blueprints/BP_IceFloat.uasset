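; Floating ice platform that bobs and tilts on a looked-up timeline, starting after a random delay.
; Its collider lowers an overlapping character's friction and braking, restores them on exit, and calls BreakObject if another overlap begins while occupied.
; BreakEvent sinks the floe and stops the bobbing; RespawnEvent animates height between saved Z and MinusZ, then calls RespawnObject and restarts bobbing.
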(event OnComponentBeginOverlap(IceCollider)
  (params (OverlappedComponent :type Primitive%20Component%20Object%20Reference) (OtherActor :type Actor%20Object%20Reference) (OtherComp :type Primitive%20Component%20Object%20Reference) (OtherBodyIndex :type Integer) (bFromSweep :type Boolean) (SweepResult :type Hit%20Result%20Structure%20%28by%20ref%29))
  (bind _ascharacter_base (Utilities|Casting|CastToCharacterBase OtherActor))
  (Utilities|FlowControl|Sequence
    (:then_0
      (Variables|/Script/Engine.CharacterMovementComponent|SetGroundFriction (Variables|/Script/Engine.Character|GetCharacterMovement _ascharacter_base) 6.0)
      (Variables|/Script/Engine.CharacterMovementComponent|SetBrakingDecelerationWalking (Variables|/Script/Engine.Character|GetCharacterMovement _ascharacter_base) 1.5e+03))
    (:then_1
      (if (Variables|Default|GetActorIsOnPlatform)
        (Variables|Default|SetActorIsOnPlatform false)
        (Class|IceFloat|BreakObject)
        (else
          (Variables|Default|SetActorIsOnPlatform true))))))

(event OnComponentEndOverlap(IceCollider)
  (params (OverlappedComponent :type Primitive%20Component%20Object%20Reference) (OtherActor :type Actor%20Object%20Reference) (OtherComp :type Primitive%20Component%20Object%20Reference) (OtherBodyIndex :type Integer))
  (Utilities|FlowControl|Sequence
    (:then_0
      (bind _ascharacter_base (Utilities|Casting|CastToCharacterBase OtherActor))
      (Utilities|FlowControl|Sequence
        (:then_0
          (Variables|/Script/Engine.CharacterMovementComponent|SetGroundFriction (Variables|/Script/Engine.Character|GetCharacterMovement _ascharacter_base) 8.0)
          (Variables|/Script/Engine.CharacterMovementComponent|SetBrakingDecelerationWalking (Variables|/Script/Engine.Character|GetCharacterMovement _ascharacter_base) 2e+03))))
    (:then_1
      (Variables|Default|SetActorIsOnPlatform false))))

(event EventRespawnEvent
  (bind _returnvalue (Transformation|GetActorLocation))
  (bind _returnvalue_2 (Transformation|GetActorLocation))
  (bind _returnvalue_3 (Transformation|GetActorLocation))
  (bind (_x _y _z) (Math|Vector|BreakVector _returnvalue))
  (bind (_x_2 _y_2) (Math|Vector|BreakVector _returnvalue_2))
  (bind _height (Timeline|Respawn PlayFromStart)
    (:Update
      (Transformation|SetActorLocation (Math|Vector|Lerp(Vector) (Math|Vector|MakeVector (.x _returnvalue_3) (.y _returnvalue_3) (Variables|Default|GetsavedOrgZ)) (Math|Vector|MakeVector _x_2 _y_2 (Variables|Default|GetMinusZ)) _height) false false))
    (:Finished
      (Class|IceFloat|RespawnObject)
      (bind (_direction _height_2 _rotationx _rotationy) (Timeline|IceFloatTImeline PlayFromStart)
        (:Update
          (Utilities|FlowControl|Sequence
            (:then_0
              (Transformation|SetActorLocation (Math|Vector|Lerp(Vector) (Variables|Default|GetOrgActorLocation) (Math|Vector|MakeVector _x _y (- _z 5.0)) _height_2) false false))
            (:then_1
              (Transformation|SetActorRotation (Math|Rotator|MakeRotator _rotationx _rotationy (.Yaw (Math|Rotator|BreakRotator (Variables|Default|GetOrgActorRotation))))))))))))

(event EventBreakEvent
  (bind _returnvalue (Transformation|GetActorLocation))
  (bind _returnvalue_2 (Transformation|GetActorLocation))
  (bind (_x _y _z) (Math|Vector|BreakVector _returnvalue))
  (bind (_x_2 _y_2 _z_2) (Math|Vector|BreakVector _returnvalue_2))
  (bind _height (Timeline|SinkTimeline PlayFromStart)
    (:Update
      (Utilities|FlowControl|Sequence
        (:then_0
          (Transformation|SetActorLocation (Math|Vector|Lerp(Vector) (Transformation|GetActorLocation) (Math|Vector|MakeVector _x_2 _y_2 (- _z_2 5.0)) _height) false false))
        (:then_1
          (bind (_direction _height_2 _rotationx _rotationy) (Timeline|IceFloatTImeline Stop)
            (:Update
              (Utilities|FlowControl|Sequence
                (:then_0
                  (Transformation|SetActorLocation (Math|Vector|Lerp(Vector) (Variables|Default|GetOrgActorLocation) (Math|Vector|MakeVector _x _y (- _z 5.0)) _height_2) false false))
                (:then_1
                  (Transformation|SetActorRotation (Math|Rotator|MakeRotator _rotationx _rotationy (.Yaw (Math|Rotator|BreakRotator (Variables|Default|GetOrgActorRotation))))))))))))))

(event EventBeginPlay
  (bind _returnvalue (Transformation|GetActorLocation))
  (bind (_x _y _z) (Math|Vector|BreakVector _returnvalue))
  (Utilities|FlowControl|Sequence
    (:then_0
      (Variables|Default|SetsavedOrgZ (.z (Transformation|GetActorLocation))))
    (:then_1
      (Utilities|FlowControl|Delay (Math|Random|RandomFloatinRange 0.0 4.0))
      (bind (_direction _height _rotationx _rotationy) (Timeline|IceFloatTImeline PlayFromStart)
        (:Update
          (Utilities|FlowControl|Sequence
            (:then_0
              (Transformation|SetActorLocation (Math|Vector|Lerp(Vector) (Variables|Default|GetOrgActorLocation) (Math|Vector|MakeVector _x _y (- _z 5.0)) _height) false false))
            (:then_1
              (Transformation|SetActorRotation (Math|Rotator|MakeRotator _rotationx _rotationy (.Yaw (Math|Rotator|BreakRotator (Variables|Default|GetOrgActorRotation))))))))))
    (:then_2
      (Variables|Default|SetOrgActorLocation (Transformation|GetActorLocation)))
    (:then_3
      (Variables|Default|SetOrgActorRotation (Transformation|GetActorRotation)))))

(fn ConstructionScript)