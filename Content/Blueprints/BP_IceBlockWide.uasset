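; BP_IceBlockWide is a wide ice block that can be pushed or pulled through an interaction showing a hold-button prompt.
; Interact and EndInteraction hand the movement to the interactor by calling its BeginPush and EndPush.
; While the block is tagged Grabbed, Tick runs a short downward box trace from its PhysicsConstraint and flags PushableProperties as falling when nothing is hit, with debug drawing left on.
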(event Collision|EventActorBeginOverlap
  (params (OtherActor :type Actor%20Object%20Reference)))

(event EventTick
  (params (DeltaSeconds :type Float%20%28single-precision%29))
  (bind _pushableproperties (Variables|Default|GetPushableProperties))
  (bind _physicsconstraint (Variables|Default|GetPhysicsConstraint))
  (bind _returnvalue (Transformation|GetWorldLocation _physicsconstraint))
  (if (Actor|ActorHasTag "Grabbed")
    (bind _returnvalue_2 (Class|KismetSystemLibrary|BoxTraceSinglebyProfile _returnvalue (- _returnvalue "0.000000,0.000000,20.000000") "165.000000,165.000000,0.000000" "0, 0, 0" "BlockAllDynamic" false 0 "ForOneFrame" true))
    (if _returnvalue_2
      (Variables|/Script/SPM.PushableProperties|SetbIsFalling _pushableproperties false)
      (else
        (Variables|/Script/SPM.PushableProperties|SetbIsFalling _pushableproperties true)))))

(fn ConstructionScript)

(fn GetPopupImage
  (return 0))

(fn GetPopupText
  (return ""))

(fn GetPopupInfo
  (params (Interactor :type Character%20Base%20Object%20Reference))
  (return "Hold To Push/Pull" "/Game/Assets/UI/Buttons/Controller/ButtonX_70x70.ButtonX_70x70"))

(fn Interact
  (params (Interactor :type Character%20Base%20Object%20Reference))
  (Class|CharacterBase|BeginPush Interactor)
  (return false))

(fn EndInteraction
  (params (Interactor :type Character%20Base%20Object%20Reference))
  (Class|CharacterBase|EndPush Interactor)
  (return false))