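; BP_GrabTestCube_Wide is a wide test cube for grabbing and pushing that tracks whether it is falling.
; Each tick, a wide, flat box trace runs a short distance down from the PhysicsConstraint, setting IsFalling on PushableProperties when nothing blocking is hit and clearing it otherwise.
; Popup getters supply MyPopupText as the text and leave the image unset.
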(event Collision|EventActorBeginOverlap
  (params (OtherActor :type Actor%20Object%20Reference)))

(event EventTick
  (params (DeltaSeconds :type Float%20%28single-precision%29))
  (bind _pushableproperties (Variables|Default|GetPushableProperties))
  (bind _physicsconstraint (Variables|Default|GetPhysicsConstraint))
  (bind _returnvalue (Transformation|GetWorldLocation _physicsconstraint))
  (bind _returnvalue_2 (Class|KismetSystemLibrary|BoxTraceSinglebyProfile _returnvalue (- _returnvalue "0.000000,0.000000,10.000000") "160.000000,160.000000,0.000000" "0, 0, 0" "BlockAllDynamic" false 0 "None" true))
  (if _returnvalue_2
    (Variables|/Script/SPM.PushableProperties|SetbIsFalling _pushableproperties false)
    (else
      (Variables|/Script/SPM.PushableProperties|SetbIsFalling _pushableproperties true))))

(fn ConstructionScript)

(fn GetPopupImage
  (return 0))

(fn GetPopupText
  (return (Variables|Default|GetMyPopupText)))