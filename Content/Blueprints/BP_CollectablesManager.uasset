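; BP_CollectablesManager tracks how many collectables have been picked up.
; Its Collected event increments NumberCollected and prints TotalCollectables, a slash and the new count as separate debug strings.
; A comparison of the count against the total is present but not connected, so completion triggers nothing.
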(event Custom|Collected
  (Variables|Default|SetNumberCollected (+ (Variables|Default|GetNumberCollected) 1.0))
  (Development|PrintString (Utilities|String|ToString(Float) (Variables|Default|GetTotalCollectables)))
  (Development|PrintString "/")
  (Development|PrintString (Utilities|String|ToString(Float) (Variables|Default|GetNumberCollected))))

(fn ConstructionScript)