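; BP_MiniGameManager tracks the win condition of a press-based minigame and starts the victory sequence.
; On Tick it compares CorrectPresses to CorrectPressesToWin, latches a Victory flag on a match, then triggers VictoryCutscene after a short delay.
; A separate MovePlayers function snaps a player character to a victory character's location and rotation and disables that player's input.
; Neither the press counting nor any call to MovePlayers happens in this Blueprint.
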(event EventTick
  (params (DeltaSeconds :type Float%20%28single-precision%29))
  (if (not (Variables|Default|GetVictory))
    (if (== (Variables|Default|GetCorrectPresses) (Variables|Default|GetCorrectPressesToWin))
      (Variables|Default|SetVictory true)
      (Utilities|FlowControl|Delay 1.0)
      (Default|TriggerVictory (Variables|Default|GetVictoryCutscene)))))

(fn ConstructionScript)

(fn MovePlayers
  (params (PlayerCharacter :type Character%20Object%20Reference) (VictoryCharacter :type Actor%20Object%20Reference))
  (Transformation|SetActorLocationAndRotation PlayerCharacter (Transformation|GetActorLocation VictoryCharacter) (Transformation|GetActorRotation VictoryCharacter))
  (bind _asbp_character_player_controller (Utilities|Casting|CastToBP_CharacterPlayerController (Pawn|GetController PlayerCharacter)))
  (Input|DisableInput PlayerCharacter _asbp_character_player_controller))