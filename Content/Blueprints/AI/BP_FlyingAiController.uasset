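; AI controller for BP_FlyingAi that runs the BT_FlyingAI behavior tree and reacts to sensing the player.
; Perception updates filter for actors tagged PlayerBig, store the stimulus as ActiveSense and route index 0 to SightSense.
; A successful sighting records stimulus and receiver locations, switches the pawn's AiState and sets its max fly speed.
; A failed sighting switches AiState back but leaves the speed unchanged.
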(event OnPerceptionUpdated(AIPerception)
  (params (UpdatedActors :type Array%20of%20Actor%20Object%20References))
  (for (_array_element _array_index) UpdatedActors
    (if (Actor|ActorHasTag _array_element "PlayerBig")
      (bind _info (Class|AIPerceptionComponent|GetActorsPerception (Variables|Default|GetAIPerception) _array_element))
      (for _array_element_2 (.lastsensedstimuli _info)
        (Variables|Default|SetActive%20Sense _array_element_2)
        (switch int _array_index
          (:0
            (CallFunction|SightSense)))))))

(event Custom|SightSense
  (bind _active_sense (Variables|Default|GetActive%20Sense))
  (bind (_age _expirationage _strength _stimuluslocation _receiverlocation _tag _bsuccessfullysensed) (Utilities|Struct|BreakAIStimulus _active_sense))
  (if _bsuccessfullysensed
    (Variables|Default|SetStimulus%20Location _stimuluslocation)
    (Variables|Default|SetReceiver%20Location _receiverlocation)
    (Development|PrintString "Player On Sight")
    (Variables|/Game/Blueprints/BP_FlyingAi.BP_FlyingAi_C|SetAiState (Variables|Default|GetFlying%20Ai%20ref) "NewEnumerator1")
    (Variables|/Script/Engine.CharacterMovementComponent|SetMaxFlySpeed (Variables|/Script/Engine.Character|GetCharacterMovement (Variables|Default|GetFlying%20Ai%20ref)) 6e+02)
    (else
      (Variables|/Game/Blueprints/BP_FlyingAi.BP_FlyingAi_C|SetAiState (Variables|Default|GetFlying%20Ai%20ref) "NewEnumerator0"))))

(event EventBeginPlay
  (AI|RunBehaviorTree "/Game/AI/BT_FlyingAI.BT_FlyingAI")
  (bind _asbp_flying_ai (Utilities|Casting|CastToBP_FlyingAi (Pawn|GetControlledPawn)))
  (Variables|Default|SetFlying%20Ai%20ref _asbp_flying_ai))

(fn ConstructionScript)