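; BP_CharSmallMainMenu is the small character displayed in the main menu, looping a waving help animation.
; On BeginPlay it caches the WarmerTogether game instance and binds to its settings-updated event.
; That event and the initial setup both apply the player's saved small-character customization through the Customize component's material index.
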(event Custom|ColorUpdated
  (Class|CustomizeComponent|SetMaterialbyIndex (Variables|Default|GetCustomize) (.customizationsmall (Variables|/Game/Blueprints/SaveGame/BP_WarmerTogetherGameInstance.BP_WarmerTogetherGameInstance_C|GetPlayerSettings (Variables|Default|GetAs%20BP%20Warmer%20Together%20Game%20Instance)))))

(event EventBeginPlay
  (Components|Animation|PlayAnimation (Variables|Default|GetSkeletalMesh) "/Game/Characters/SmallCharacter/Animations/AC_SmallWaveHelp.AC_SmallWaveHelp" true)
  (bind _asbp_warmer_together_game_instance (Utilities|Casting|CastToBP_WarmerTogetherGameInstance (Game|GetGameInstance)))
  (bind _output_get (Variables|Default|SetAs%20BP%20Warmer%20Together%20Game%20Instance _asbp_warmer_together_game_instance))
  (EventDispatchers|BindEventtoSettingsHaveUpdated _output_get (delegate Custom|ColorUpdated))
  (CallFunction|ColorUpdated))

(fn ConstructionScript)