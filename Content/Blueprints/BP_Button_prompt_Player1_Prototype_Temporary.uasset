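; Temporary prototype button prompt that shows in-world text when the big character (BP_CharacterBig) enters its trigger box.
; Box overlap events cast to that character class, revealing the TextRender on entry and hiding it on exit.
; When PromptType is 1, the text is replaced with the Text variable before showing; otherwise the component's existing text is shown.
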(event OnComponentBeginOverlap(Box)
  (params (OverlappedComponent :type Primitive%20Component%20Object%20Reference) (OtherActor :type Actor%20Object%20Reference) (OtherComp :type Primitive%20Component%20Object%20Reference) (OtherBodyIndex :type Integer) (bFromSweep :type Boolean) (SweepResult :type Hit%20Result%20Structure%20%28by%20ref%29))
  (Utilities|Casting|CastToBP_CharacterBig OtherActor)
  (if (== 1 (Variables|Default|GetPromptType))
    (Rendering|Components|TextRender|SetText (Variables|Default|GetTextRender) (Variables|Default|GetText))
    (Development|SetHiddeninGame (Variables|Default|GetTextRender) false false)
    (else
      (Development|SetHiddeninGame (Variables|Default|GetTextRender) false false))))

(event OnComponentEndOverlap(Box)
  (params (OverlappedComponent :type Primitive%20Component%20Object%20Reference) (OtherActor :type Actor%20Object%20Reference) (OtherComp :type Primitive%20Component%20Object%20Reference) (OtherBodyIndex :type Integer))
  (Utilities|Casting|CastToBP_CharacterBig OtherActor)
  (Development|SetHiddeninGame (Variables|Default|GetTextRender) true false))

(fn ConstructionScript)