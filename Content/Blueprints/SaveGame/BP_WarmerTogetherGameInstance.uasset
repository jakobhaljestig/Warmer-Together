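; Game instance for WarmerTogether that persists Settings and the current level in a single BP_SaveGame slot.
; Init creates the save if none exists, and LoadGame falls back to saving when the slot is missing.
; Saves write a fresh object asynchronously.
; Async loading copies values on the immediate exec pin rather than Completed, which only triggers the settings-updated notification.
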(event Custom|SaveGame
  ;[0.15 0.15 0.15 0.5] SaveGame
  (bind _returnvalue (SaveGame|CreateSaveGameObject "/Game/Blueprints/SaveGame/BP_SaveGame.BP_SaveGame_C"))
  (bind _output_get (Variables|Default|SetSaveGameInstance _returnvalue))
  (Variables|/Game/Blueprints/SaveGame/BP_SaveGame.BP_SaveGame_C|SetSettings _output_get (Variables|Default|GetSettings))
  (Variables|/Game/Blueprints/SaveGame/BP_SaveGame.BP_SaveGame_C|SetCurrentLevel _output_get (Variables|Default|GetCurrentLevel))
  (|AsyncSaveGametoSlot _output_get (Variables|Default|GetSaveGameSlotName)))

(event Custom|SettingsHaveBeenUpdated
  (Default|CallSettingsHasUpdated))

(event Custom|LoadGame
  ;[0.15 0.15 0.15 0.5] LoadGame
  (bind _returnvalue (SaveGame|DoesSaveGameExist (Variables|Default|GetSaveGameSlotName)))
  (if _returnvalue
    (bind _savegame (|AsyncLoadGamefromSlot (Variables|Default|GetSaveGameSlotName))
      (:then
        (bind _asbp_save_game (Utilities|Casting|CastToBP_SaveGame _savegame))
        (Variables|Default|SetSettings (Variables|/Game/Blueprints/SaveGame/BP_SaveGame.BP_SaveGame_C|GetSettings _asbp_save_game))
        (Variables|Default|SetCurrentLevel (Variables|/Game/Blueprints/SaveGame/BP_SaveGame.BP_SaveGame_C|GetCurrentLevel _asbp_save_game)))
      (:Completed
        (CallFunction|SettingsHaveBeenUpdated)))
    (else
      (CallFunction|SaveGame))))

(event EventInit
  ;[0.15 0.15 0.15 0.5] Initialization
  (bind _returnvalue (SaveGame|DoesSaveGameExist (Variables|Default|GetSaveGameSlotName)))
  (if (not _returnvalue)
    (CallFunction|SaveGame)))