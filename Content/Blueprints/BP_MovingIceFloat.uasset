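; Ice float platform that makes characters slide and can break, sink and respawn.
; Its collider lowers character friction and braking on overlap, then sets higher values on exit.
; A character overlap while the occupied flag is already set calls BreakObject.
; BreakEvent's timeline nudges the float downward, while RespawnEvent's timeline interpolates height between saved start Z and MinusZ, then calls RespawnObject.
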(event OnComponentBeginOverlap(IceCollider)
  (params (OverlappedComponent :type Primitive%20Component%20Object%20Reference) (OtherActor :type Actor%20Object%20Reference) (OtherComp :type Primitive%20Component%20Object%20Reference) (OtherBodyIndex :type Integer) (bFromSweep :type Boolean) (SweepResult :type Hit%20Result%20Structure%20%28by%20ref%29))
  (bind _ascharacter_base (Utilities|Casting|CastToCharacterBase OtherActor))
  (Utilities|FlowControl|Sequence
    (:then_0
      (Variables|/Script/Engine.CharacterMovementComponent|SetGroundFriction (Variables|/Script/Engine.Character|GetCharacterMovement _ascharacter_base) 6.0)
      (Variables|/Script/Engine.CharacterMovementComponent|SetBrakingDecelerationWalking (Variables|/Script/Engine.Character|GetCharacterMovement _ascharacter_base) 1.5e+03))
    (:then_1
      (if (Variables|Default|GetActorIsOnPlatform)
        (Variables|Default|SetActorIsOnPlatform false)
        (Class|IceFloat|BreakObject)
        (else
          (Variables|Default|SetActorIsOnPlatform true))))))

(event OnComponentEndOverlap(IceCollider)
  (params (OverlappedComponent :type Primitive%20Component%20Object%20Reference) (OtherActor :type Actor%20Object%20Reference) (OtherComp :type Primitive%20Component%20Object%20Reference) (OtherBodyIndex :type Integer))
  (Utilities|FlowControl|Sequence
    (:then_0
      (bind _ascharacter_base (Utilities|Casting|CastToCharacterBase OtherActor))
      (Variables|/Script/Engine.CharacterMovementComponent|SetGroundFriction (Variables|/Script/Engine.Character|GetCharacterMovement _ascharacter_base) 8.0)
      (Variables|/Script/Engine.CharacterMovementComponent|SetBrakingDecelerationWalking (Variables|/Script/Engine.Character|GetCharacterMovement _ascharacter_base) 2e+03))
    (:then_1
      (Variables|Default|SetActorIsOnPlatform false))))

(event EventRespawnEvent
  (bind _returnvalue (Transformation|GetActorLocation))
  (bind _returnvalue_2 (Transformation|GetActorLocation))
  (bind (_x _y) (Math|Vector|BreakVector _returnvalue))
  (bind _height (Timeline|Timeline_0 PlayFromStart)
    (:Update
      (Transformation|SetActorLocation (Math|Vector|Lerp(Vector) (Math|Vector|MakeVector (.x _returnvalue_2) (.y _returnvalue_2) (Variables|Default|GetsavedOrgZ)) (Math|Vector|MakeVector _x _y (Variables|Default|GetMinus%20Z)) _height) false false))
    (:Finished
      (Class|IceFloat|RespawnObject))))

(event EventBreakEvent
  (bind _returnvalue (Transformation|GetActorLocation))
  (bind (_x _y _z) (Math|Vector|BreakVector _returnvalue))
  (bind _height (Timeline|Timeline PlayFromStart)
    (:Update
      (Transformation|SetActorLocation (Math|Vector|Lerp(Vector) (Transformation|GetActorLocation) (Math|Vector|MakeVector _x _y (- _z 1.0)) _height) false false))))

(event EventBeginPlay
  (Variables|Default|SetsavedOrgZ (.z (Transformation|GetActorLocation))))

(event EventTick
  (params (DeltaSeconds :type Float%20%28single-precision%29))
  (Variables|Default|SetFloatSavedLocation (Transformation|GetActorLocation)))

(fn ConstructionScript)