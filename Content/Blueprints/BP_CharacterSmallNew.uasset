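; Character Blueprint for the small player, handling its HUD prompts, freeze feedback and death from being bonked.
; Overlapping actors with either interactable interface adds or removes their popups on the HUD.
; Tick feeds body temperature into the freeze material of player controller index 1 and toggles an escape prompt based on the "Grabbed" tag.
; A moving falling tree or grab cube entering BonkBox plays a sound, launches the character backward and triggers death.
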(event OnComponentBeginOverlap(BonkBox)
  (params (OverlappedComponent :type Primitive%20Component%20Object%20Reference) (OtherActor :type Actor%20Object%20Reference) (OtherComp :type Primitive%20Component%20Object%20Reference) (OtherBodyIndex :type Integer) (bFromSweep :type Boolean) (SweepResult :type Hit%20Result%20Structure%20%28by%20ref%29))
  ;[0.15 0.15 0.15 0.5] Bonk
  (Utilities|FlowControl|Sequence
    (:then_0
      (bind _asbp_falling_tree_6 (Utilities|Casting|CastToBP_FallingTree6 OtherActor))
      (bind _returnvalue2 (Default|HasRotationChangedfromLastTick _asbp_falling_tree_6))
      (if _returnvalue2
        (if (not (Variables|Default|GetbHasDied)) :!label _label
          (Audio|PlaySound2D 0 1.0 1.0 0.0 0 0)
          (Character|LaunchCharacter (* (Transformation|GetActorForwardVector) "-1000.000000,-0.000000,0.000000") false false)
          (Class|CharacterBase|OnDeath))))
    (:then_1
      (bind _asbp_grab_test_cube (Utilities|Casting|CastToBP_GrabTestCube OtherActor))
      (if (> (Math|Vector|VectorLength (Transformation|GetVelocity _asbp_grab_test_cube)) 1.0)
        (goto _label)))))

(event Collision|EventActorBeginOverlap
  (params (OtherActor :type Actor%20Object%20Reference))
  (bind _as_wb_hud (Variables|Default|GetAs%20WB%20HUD))
  ;[0.2829 0.776 0.4547 0.5] Player has entered collider of interactable object
  (Utilities|FlowControl|Sequence
    (:then_0
      (bind _asbi_interactable (Utilities|Casting|CastToBI_Interactable OtherActor))
      (bind (_popuptext _popupimage) (Default|GetPopupInfo _asbi_interactable))
      (Default|AddPopup _as_wb_hud _popuptext _popupimage))
    (:then_1
      (bind _asbi_character_small_interactable (Utilities|Casting|CastToBI_CharacterSmallInteractable OtherActor))
      (bind (_popuptext_2 _popupimage_2) (Default|GetPopupInfo _asbi_character_small_interactable))
      (Default|AddPopup _as_wb_hud _popuptext_2 _popupimage_2))))

(event EventTick
  (params (DeltaSeconds :type Float%20%28single-precision%29))
  (bind _as_wb_hud (Variables|Default|GetAs%20WB%20HUD))
  ;[0.15 0.15 0.15 0.5] Freeze effect in HUD
  (bind _ascharacter_player_controller (Utilities|Casting|CastToCharacterPlayerController (Game|GetPlayerController 1)))
  (bind _aswb_freeze_effect (Utilities|Casting|CastToWB_FreezeEffect (Variables|/Script/SPM.CharacterPlayerController|GetFreezeEffect _ascharacter_player_controller)))
  (Rendering|Material|SetScalarParameterValue (Variables|/Game/Blueprints/UI/WB_FreezeEffect.WB_FreezeEffect_C|GetFreezeMaterialInstance _aswb_freeze_effect) "FreezeIntensity" (Variables|/Script/SPM.BodyTemperature|GetTemperaturePrecent (Variables|Default|GetBodyTempComponent)) :!class /Script/Engine.MaterialInstanceDynamic)
  ;[0.2829 0.776 0.4547 0.5] Small player is picked up by big player (popup)
  (if (Actor|ActorHasTag "Grabbed")
    (Default|AddPopup _as_wb_hud "Press To Escape" "/Game/Assets/UI/Buttons/Controller/ButtonB_70x70.ButtonB_70x70")
    (Variables|Default|SetPopupIsCreated true)
    (elif (Variables|Default|GetPopupIsCreated)
      (Default|RemovePopupbyText _as_wb_hud "Press To Escape")
      (Variables|Default|SetPopupIsCreated false))))

(event Collision|EventActorEndOverlap
  (params (OtherActor :type Actor%20Object%20Reference))
  (bind _as_wb_hud (Variables|Default|GetAs%20WB%20HUD))
  ;[0.15 0.02847 0.04493 0.5] Player has exited collider of interactable object
  (Utilities|FlowControl|Sequence
    (:then_0
      (bind _asbi_interactable (Utilities|Casting|CastToBI_Interactable OtherActor))
      (bind _popuptext (Default|GetPopupInfo _asbi_interactable))
      (Default|RemovePopupbyText _as_wb_hud _popuptext))
    (:then_1
      (bind _asbi_character_small_interactable (Utilities|Casting|CastToBI_CharacterSmallInteractable OtherActor))
      (bind _popuptext_2 (Default|GetPopupInfo _asbi_character_small_interactable))
      (Default|RemovePopupbyText _as_wb_hud _popuptext_2))))

(fn ConstructionScript)