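; Actor that applies the player's saved audio volume settings to the game's sound classes.
; On BeginPlay it caches the WarmerTogether game instance, binds to its settings-updated event and applies the volumes immediately.
; Each update overrides the Music, Effects and Ambient class volumes in the main sound mix from PlayerSettings, pushing the mix after each override.
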(event Custom|VolumeUpdated
  (bind _as_bp_warmer_together_game_instance (Variables|Default|GetAs%20BP%20Warmer%20Together%20Game%20Instance))
  (bind _playersettings (Variables|/Game/Blueprints/SaveGame/BP_WarmerTogetherGameInstance.BP_WarmerTogetherGameInstance_C|GetPlayerSettings _as_bp_warmer_together_game_instance))
  (Utilities|FlowControl|Sequence
    (:then_0
      (Audio|SetSoundMixClassOverride "/Game/Audio/SCM_MainSoundMix.SCM_MainSoundMix" "/Game/Audio/SFX_Music.SFX_Music" (.musicvolume _playersettings) 1.0 1.0 true)
      (Audio|PushSoundMixModifier "/Game/Audio/SCM_MainSoundMix.SCM_MainSoundMix"))
    (:then_1
      (Audio|SetSoundMixClassOverride "/Game/Audio/SCM_MainSoundMix.SCM_MainSoundMix" "/Game/Audio/SFX_Effects.SFX_Effects" (.effectsvolume _playersettings) 1.0 1.0 true)
      (Audio|PushSoundMixModifier "/Game/Audio/SCM_MainSoundMix.SCM_MainSoundMix"))
    (:then_2
      (Audio|SetSoundMixClassOverride "/Game/Audio/SCM_MainSoundMix.SCM_MainSoundMix" "/Game/Audio/SFX_Ambient.SFX_Ambient" (.ambiancevolume _playersettings) 1.0 1.0 true)
      (Audio|PushSoundMixModifier "/Game/Audio/SCM_MainSoundMix.SCM_MainSoundMix"))))

(event EventBeginPlay
  (bind _asbp_warmer_together_game_instance (Utilities|Casting|CastToBP_WarmerTogetherGameInstance (Game|GetGameInstance)))
  (bind _output_get (Variables|Default|SetAs%20BP%20Warmer%20Together%20Game%20Instance _asbp_warmer_together_game_instance))
  (EventDispatchers|BindEventtoSettingsHaveUpdated _output_get (delegate Custom|VolumeUpdated))
  (CallFunction|VolumeUpdated))

(fn ConstructionScript)