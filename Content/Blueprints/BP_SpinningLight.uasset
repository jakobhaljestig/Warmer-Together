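; BP_SpinningLight is an actor with a spotlight that continuously spins and orbits the actor's starting location.
; BeginPlay caches the actor location, and each Tick adds a fixed world yaw to the SpotLight and places it along its forward vector at Distance from that point.
; The rotation step is per frame and not scaled by delta time, so spin speed depends on frame rate.
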(event EventBeginPlay
  (Variables|Default|SetStartLocation (Transformation|GetActorLocation)))

(event Collision|EventActorBeginOverlap
  (params (OtherActor :type Actor%20Object%20Reference)))

(event EventTick
  (params (DeltaSeconds :type Float%20%28single-precision%29))
  (bind _spotlight (Variables|Default|GetSpotLight))
  (Transformation|AddWorldRotation (Variables|Default|GetSpotLight) (Math|Rotator|MakeRotator 0.0 0.0 1.0) false false)
  (Transformation|SetWorldLocation _spotlight (+ (Variables|Default|GetStartLocation) (* (Math|Vector|GetForwardVector _spotlight) (Variables|Default|GetDistance))) false false))

(fn ConstructionScript)