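; BP_CharacterBig is the big character Blueprint, handling on-screen button prompts for its interactions.
; Begin overlap casts the other actor to cubes, falling trees, ladder colliders, the radio tower or the small character, creating push/pull, climb or pick-up/hug popups that end overlap removes.
; Tick polls the IsLifting tag, using a WidgetIsCreated flag to show and remove a throw prompt.
; An unconnected copy of the throw-prompt logic never runs.
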(event Collision|EventActorBeginOverlap
  (params (OtherActor :type Actor%20Object%20Reference))
  (Utilities|FlowControl|Sequence
    (:then_0
      (Utilities|Casting|CastToBP_GrabTestCube OtherActor)
      (bind _returnvalue (UserInterface|CreateWidget "/Game/UI_Assets/WBP_PopupWidget.WBP_PopupWidget_C" :!label _label))
      (Variables|/Game/UI_Assets/WBP_PopupWidget.WBP_PopupWidget_C|SetPopupText _returnvalue "Hold To Push/Pull")
      (Variables|/Game/UI_Assets/WBP_PopupWidget.WBP_PopupWidget_C|SetPopupImage _returnvalue "/Game/UI_Assets/Buttons/Controller/L2.L2")
      (UserInterface|Viewport|AddtoPlayerScreen _returnvalue))
    (:then_1
      (Utilities|Casting|CastToBP_FallingTree6 OtherActor)
      (goto _label))
    (:then_2
      (Utilities|Casting|CastToBP_PopupLadderCollider OtherActor)
      (bind _returnvalue_2 (UserInterface|CreateWidget "/Game/UI_Assets/WBP_PopupWidget.WBP_PopupWidget_C" :!label _label_2))
      (Variables|/Game/UI_Assets/WBP_PopupWidget.WBP_PopupWidget_C|SetPopupText _returnvalue_2 "Press To Climb")
      (Variables|/Game/UI_Assets/WBP_PopupWidget.WBP_PopupWidget_C|SetPopupImage _returnvalue_2 "/Game/UI_Assets/Buttons/Controller/ButtonX_70x70.ButtonX_70x70")
      (UserInterface|Viewport|AddtoPlayerScreen _returnvalue_2))
    (:then_3
      (Utilities|Casting|CastToBP_RadioTower OtherActor)
      (goto _label_2))
    (:then_4
      (Utilities|Casting|CastToBP_CharacterSmallNew OtherActor)
      (bind _returnvalue_3 (UserInterface|CreateWidget "/Game/UI_Assets/WBP_PlayerPopupWidget1.WBP_PlayerPopupWidget1_C"))
      (Variables|/Game/UI_Assets/WBP_PlayerPopupWidget1.WBP_PlayerPopupWidget1_C|SetPopupText _returnvalue_3 "Press To Pick Up")
      (Variables|/Game/UI_Assets/WBP_PlayerPopupWidget1.WBP_PlayerPopupWidget1_C|SetPopupImage _returnvalue_3 "/Game/UI_Assets/Buttons/Controller/ButtonB_70x70.ButtonB_70x70")
      (Variables|/Game/UI_Assets/WBP_PlayerPopupWidget1.WBP_PlayerPopupWidget1_C|SetPopupImage2 _returnvalue_3 "/Game/UI_Assets/Buttons/Controller/ButtonX_70x70.ButtonX_70x70")
      (Variables|/Game/UI_Assets/WBP_PlayerPopupWidget1.WBP_PlayerPopupWidget1_C|SetPopupText2 _returnvalue_3 "Hold To Hug")
      (UserInterface|Viewport|AddtoPlayerScreen _returnvalue_3))))

(event EventTick
  (params (DeltaSeconds :type Float%20%28single-precision%29))
  (bind _returnvalue (Actor|ActorHasTag "IsLifting"))
  (if (Variables|Default|GetWidgetIsCreated)
    (if (and (Variables|Default|GetWidgetIsCreated) (not _returnvalue))
      (Widget|RemovefromParent (stale _output_get))
      (Variables|Default|SetWidgetIsCreated false))
    (elif _returnvalue
      (bind _returnvalue_2 (UserInterface|CreateWidget "/Game/UI_Assets/WBP_PopupWidget.WBP_PopupWidget_C"))
      (Variables|Default|SetWidgetIsCreated true)
      (bind _output_get (Variables|Default|SetWidget _returnvalue_2))
      (Variables|/Game/UI_Assets/WBP_PopupWidget.WBP_PopupWidget_C|SetPopupText _returnvalue_2 "Press To Throw")
      (Variables|/Game/UI_Assets/WBP_PopupWidget.WBP_PopupWidget_C|SetPopupImage _returnvalue_2 "/Game/UI_Assets/Buttons/Controller/ButtonB_70x70.ButtonB_70x70")
      (UserInterface|Viewport|AddtoPlayerScreen _returnvalue_2))))

(event Collision|EventActorEndOverlap
  (params (OtherActor :type Actor%20Object%20Reference))
  (Utilities|FlowControl|Sequence
    (:then_0
      (Utilities|Casting|CastToBP_GrabTestCube OtherActor)
      (Widget|RemovefromParent (stale Collision|EventActorBeginOverlap _returnvalue) :!label _label))
    (:then_1
      (Utilities|Casting|CastToBP_FallingTree6 OtherActor)
      (goto _label))
    (:then_2
      (Utilities|Casting|CastToBP_PopupLadderCollider OtherActor)
      (Widget|RemovefromParent (stale Collision|EventActorBeginOverlap _returnvalue_2) :!label _label_2))
    (:then_3
      (Utilities|Casting|CastToBP_RadioTower OtherActor)
      (goto _label_2))
    (:then_4
      (Utilities|Casting|CastToBP_CharacterSmallNew OtherActor)
      (Widget|RemovefromParent (stale Collision|EventActorBeginOverlap _returnvalue_3)))))

(fn ConstructionScript)