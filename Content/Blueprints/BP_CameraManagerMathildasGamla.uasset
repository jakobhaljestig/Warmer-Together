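; Camera manager that switches between shared framing and per-player views based on the distance between the big and small characters.
; Each tick below the merge threshold, it moves itself toward their midpoint with interpolation, clamping X and Y to bounds.
; Otherwise it blends player controllers 0 and 1 to their respective characters.
; The merge branch only moves the actor and never sets the view target back.
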(event EventTick
  (params (DeltaSeconds :type Float%20%28single-precision%29))
  (bind _characterbig (Variables|Default|GetCharacterBig))
  (bind _charactersmall (Variables|Default|GetCharacterSmall))
  (bind _camera (Variables|Default|GetCamera))
  (bind _maxbounds (Variables|Default|GetMaxBounds))
  (bind _minbounds (Variables|Default|GetMinBounds))
  (bind _returnvalue (Transformation|GetActorLocation _charactersmall))
  (bind _returnvalue_2 (Transformation|GetActorLocation _characterbig))
  (bind _returnvalue_3 (Transformation|GetWorldLocation _camera))
  (bind _returnvalue_4 (+ _returnvalue_2 _returnvalue))
  (bind _returnvalue_5 (/ _returnvalue_4 2.0))
  (bind _returnvalue_6 (Math|Interpolation|VInterpTo _returnvalue_3 _returnvalue_5 0.0 0.0))
  (bind (_x _y _z) (Math|Vector|BreakVector _returnvalue_6))
  (if (< (Math|Vector|VectorLength (- (Transformation|GetActorLocation (Variables|Default|GetCharacterBig)) (Transformation|GetActorLocation (Variables|Default|GetCharacterSmall)))) (Variables|Default|GetMergeThreshold))
    (Transformation|SetActorLocation (Math|Vector|MakeVector (Math|Float|Clamp(Float) _x (.x _minbounds) (.x _maxbounds)) (Math|Float|Clamp(Float) _y (.y _minbounds) (.y _maxbounds)) _z) false false)
    (else
      (Game|Player|SetViewTargetwithBlend (Game|GetPlayerController 0) (Variables|Default|GetCharacterBig) 0.5 "VTBlend_Linear" 0.0 false)
      (Game|Player|SetViewTargetwithBlend (Game|GetPlayerController 1) (Variables|Default|GetCharacterSmall) 0.5 "VTBlend_Linear" 0.0 false))))

(fn ConstructionScript)