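; Player controller that handles cold feedback and pause toggling for the CharacterBig and CharacterSmall pawns.
; Shivering events scale camera shake, HUD temperature-bar shake and rumble delay by temperature percentage, while Tick repeats the rumble; a separate event plays cold-buff rumble.
; Enter or gamepad Special Right toggles pause through the game instance: CharacterBig gets in-game settings plus a streamed Customization level, CharacterSmall a different widget.
; Unpausing unloads that level, saves and applies settings.
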(event EventTick
  (params (DeltaSeconds :type Float%20%28single-precision%29))
  (bind _as_wb_hud (Variables|Default|GetAs%20WB%20HUD))
  (if (Variables|Default|GetbCanShiver)
    (if (Variables|Default|GetIsShivering)
      (Utilities|FlowControl|Delay (Variables|Default|GetShiveringDelay))
      (Game|Feedback|ClientPlayForceFeedback "/Game/Blueprints/ForceFeedback/FFE_Shivering.FFE_Shivering" "None" false false false)
      (Class|UserWidget|SetPlaybackSpeed _as_wb_hud (Variables|/Game/Blueprints/UI/WB_HUD.WB_HUD_C|GetTempShake _as_wb_hud) (Variables|Default|GetTempBarShakeSpeed)))))

(event EventColdBuffFeedBack
  (Game|Feedback|ClientPlayForceFeedback "/Game/Blueprints/ForceFeedback/FFE_ColdBuff.FFE_ColdBuff" "None" false false false))

(event EventStartShiveringEffects
  (params (TempPercentage :type Float%20%28single-precision%29))
  (bind _returnvalue (- 1.0 TempPercentage))
  (bind _as_wb_hud (Variables|Default|GetAs%20WB%20HUD))
  (if (Variables|Default|GetbCanShiver)
    (Variables|Default|SetTempBarShakeSpeed (* _returnvalue 3.0))
    (Variables|Default|SetShiveringDelay (Math|Float|Clamp(Float) (* TempPercentage 5.0) 0.75 2.5))
    (Game|Feedback|ClientStartCameraShake "/Game/Blueprints/CameraShake/BP_CameraShakeFreezing.BP_CameraShakeFreezing_C" _returnvalue "World" "0, 0, 0")
    (if (not (Variables|Default|GetIsShivering))
      (Variables|Default|SetIsShivering true)
      (UserInterface|Animation|PlayAnimation _as_wb_hud (Variables|/Game/Blueprints/UI/WB_HUD.WB_HUD_C|GetTempShake _as_wb_hud) 0.0 0 "Forward" (Variables|Default|GetTempBarShakeSpeed) false))))

(event EventStopShiveringEffects
  (if (Variables|Default|GetbCanShiver)
    (Variables|Default|SetIsShivering false)
    (Class|UserWidget|StopAllAnimations (Variables|Default|GetAs%20WB%20HUD))
    (Game|Feedback|ClientStopCameraShake "/Game/Blueprints/CameraShake/BP_CameraShakeFreezing.BP_CameraShakeFreezing_C" false)))

(event EventBeginPlay
  (bind _asbp_warmer_together_game_instance (Utilities|Casting|CastToBP_WarmerTogetherGameInstance (Game|GetGameInstance)))
  (Variables|Default|SetAs%20BP%20Warmer%20Together%20Game%20Instance _asbp_warmer_together_game_instance))

(event Input|GamepadEvents|GamepadSpecialRight
  (params (Key :type Key%20Structure :default "None"))
  (bind _returnvalue (Pawn|GetControlledPawn))
  (bind _as_bp_warmer_together_game_instance (Variables|Default|GetAs%20BP%20Warmer%20Together%20Game%20Instance))
  ;[0.15 0.15 0.15 0.5] Pause Game
  (:Pressed
    (bind _gameshouldpause (Default|ToggleGamePaused (Variables|Default|GetAs%20BP%20Warmer%20Together%20Game%20Instance)))
    (Utilities|Casting|CastToCharacterBig _returnvalue
      (:then
        (if _gameshouldpause
          (Game|LoadStreamLevel(byName) "Customization" true)
          (bind _returnvalue_2 (UserInterface|CreateWidget "/Game/Blueprints/UI/WBP_SettingsInGame.WBP_SettingsInGame_C"))
          (bind _output_get (Variables|/Game/Blueprints/SaveGame/BP_WarmerTogetherGameInstance.BP_WarmerTogetherGameInstance_C|SetPauseWidget (Variables|Default|GetAs%20BP%20Warmer%20Together%20Game%20Instance) _returnvalue_2))
          (UserInterface|Viewport|AddtoViewport _output_get 0)
          (Game|SetGamePaused true)
          (Variables|Default|SetbShowMouseCursor true)
          (else
            (Widget|RemovefromParent (Variables|/Game/Blueprints/SaveGame/BP_WarmerTogetherGameInstance.BP_WarmerTogetherGameInstance_C|GetPauseWidget _as_bp_warmer_together_game_instance) :!label _label)
            (Game|UnloadStreamLevel(byName) "Customization" false)
            (Default|SaveGame _as_bp_warmer_together_game_instance)
            (Default|SettingsHaveBeenUpdated _as_bp_warmer_together_game_instance)
            (Game|SetGamePaused false)
            (Variables|/Script/Engine.PlayerController|SetbShowMouseCursor (Game|GetPlayerController 0) false))))
      (:CastFailed
        (Utilities|Casting|CastToCharacterSmall _returnvalue)
        (if _gameshouldpause
          (bind _returnvalue_3 (UserInterface|CreateWidget "/Game/Blueprints/UI/WBP_GamePaused.WBP_GamePaused_C"))
          (bind _output_get_2 (Variables|/Game/Blueprints/SaveGame/BP_WarmerTogetherGameInstance.BP_WarmerTogetherGameInstance_C|SetPauseWidget (Variables|Default|GetAs%20BP%20Warmer%20Together%20Game%20Instance) _returnvalue_3))
          (UserInterface|Viewport|AddtoViewport _output_get_2 0)
          (Game|SetGamePaused true)
          (else
            (goto _label)))))))

(event Input|KeyboardEvents|Enter
  (params (Key :type Key%20Structure :default "None"))
  (bind _returnvalue (Pawn|GetControlledPawn))
  (bind _as_bp_warmer_together_game_instance (Variables|Default|GetAs%20BP%20Warmer%20Together%20Game%20Instance))
  ;[0.15 0.15 0.15 0.5] Pause Game
  (:Pressed
    (bind _gameshouldpause (Default|ToggleGamePaused (Variables|Default|GetAs%20BP%20Warmer%20Together%20Game%20Instance)))
    (Utilities|Casting|CastToCharacterBig _returnvalue
      (:then
        (if _gameshouldpause
          (Game|LoadStreamLevel(byName) "Customization" true)
          (bind _returnvalue_2 (UserInterface|CreateWidget "/Game/Blueprints/UI/WBP_SettingsInGame.WBP_SettingsInGame_C"))
          (bind _output_get (Variables|/Game/Blueprints/SaveGame/BP_WarmerTogetherGameInstance.BP_WarmerTogetherGameInstance_C|SetPauseWidget (Variables|Default|GetAs%20BP%20Warmer%20Together%20Game%20Instance) _returnvalue_2))
          (UserInterface|Viewport|AddtoViewport _output_get 0)
          (Game|SetGamePaused true)
          (Variables|Default|SetbShowMouseCursor true)
          (else
            (Widget|RemovefromParent (Variables|/Game/Blueprints/SaveGame/BP_WarmerTogetherGameInstance.BP_WarmerTogetherGameInstance_C|GetPauseWidget _as_bp_warmer_together_game_instance) :!label _label)
            (Game|UnloadStreamLevel(byName) "Customization" false)
            (Default|SaveGame _as_bp_warmer_together_game_instance)
            (Default|SettingsHaveBeenUpdated _as_bp_warmer_together_game_instance)
            (Game|SetGamePaused false)
            (Variables|/Script/Engine.PlayerController|SetbShowMouseCursor (Game|GetPlayerController 0) false))))
      (:CastFailed
        (Utilities|Casting|CastToCharacterSmall _returnvalue)
        (if _gameshouldpause
          (bind _returnvalue_3 (UserInterface|CreateWidget "/Game/Blueprints/UI/WBP_GamePaused.WBP_GamePaused_C"))
          (bind _output_get_2 (Variables|/Game/Blueprints/SaveGame/BP_WarmerTogetherGameInstance.BP_WarmerTogetherGameInstance_C|SetPauseWidget (Variables|Default|GetAs%20BP%20Warmer%20Together%20Game%20Instance) _returnvalue_3))
          (UserInterface|Viewport|AddtoViewport _output_get_2 0)
          (Game|SetGamePaused true)
          (else
            (goto _label)))))))

(fn ConstructionScript)